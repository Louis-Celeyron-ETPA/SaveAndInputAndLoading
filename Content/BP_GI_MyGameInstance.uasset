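; Game instance that handles level transitions behind a loading screen and holds the current save game.
; LoadScene lazily creates and reuses the loading widget, fades it in, waits briefly, opens the level, then starts the fade out.
; InitializeSave async-loads a BP_SG_MySave, or on failure creates one with a fixed default name and ID rather than the requested ones.
; SaveGame async-writes the current save using its own name and ID.
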(event `LoadScene`
  (params (CurrenLevel :type "World Soft Object Reference"))
  (bind _loadingscreen (`self.LoadingScreen`)
    (:`then`
      _)
    (:`else`
      (bind _returnvalue (`|CreateWidget` "/Game/WBP_Loading.WBP_Loading_C"))
      (set `self.LoadingScreen` _returnvalue)))
  (`UserWidget.AddToViewport` _loadingscreen 0)
  (`/Game/WBP_Loading.LauncheFadeIn` (`self.LoadingScreen`))
  (`KismetSystemLibrary.Delay` 1.0)
  (`GameplayStatics.OpenLevelBySoftObjectPtr` CurrenLevel)
  (`/Game/WBP_Loading.LaunchFadeOut` (`self.LoadingScreen`)))

(event `SaveGame`
  (bind _currentsave (`self.CurrentSave`))
  (`AsyncActionHandleSaveGame.AsyncSaveGameToSlot` _currentsave (`/Game/BP_SG_MySave.SaveName` _currentsave) (`/Game/BP_SG_MySave.SaveID` _currentsave)))

(event `InitializeSave`
  (params (SlotName :type String) (UserIndex :type Integer))
  (bind (_savegame _bsuccess) (`AsyncActionHandleSaveGame.AsyncLoadGameFromSlot` SlotName UserIndex)
    (:`Completed`
      (if _bsuccess
        (bind _asbp_sg_my_save (cast `/Game/BP_SG_MySave` _savegame))
        (set `self.CurrentSave` _asbp_sg_my_save)
        (else
          (bind _returnvalue (`GameplayStatics.CreateSaveGameObject` "/Game/BP_SG_MySave.BP_SG_MySave_C"))
          (set `/Game/BP_SG_MySave.SaveID` 0 _returnvalue)
          (set `/Game/BP_SG_MySave.SaveName` "MainSave" _returnvalue)
          (set `self.CurrentSave` _returnvalue))))))